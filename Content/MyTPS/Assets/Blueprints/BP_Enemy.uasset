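; Zombie enemy that chases the player, attacks up close, and adds to the player's score when killed.
; Sphere overlaps toggle tracking, while Box overlaps toggle attacking, reasserted every second by a delay loop.
; Tick drives AI movement, applies damage when the AB_Zombie anim instance flags a hit, and handles death once health runs out.
; State flags are written straight to the anim instance, and death destroys the actor after a delay.
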(event `self.ReceiveBeginPlay`
  (bind _asbp_base_character (cast `/Game/MyTPS/Assets/Blueprints/BP_BaseCharacter` (`GameplayStatics.GetPlayerCharacter` 0)))
  (set `self.Player` _asbp_base_character)
  (bind _asab_zombie (cast `/Game/MyTPS/Assets/Enemy/zombie/AB_Zombie` (`SkeletalMeshComponent.GetAnimInstance` (`self.Mesh`))))
  (set `self.Enemy` _asab_zombie)
  (`KismetSystemLibrary.PrintString` "enemyinit"))

(event `self.ReceiveAnyDamage`
  (params (Damage :type "Float (single-precision)") (DamageType :type "DamageType Object Reference") (InstigatedBy :type "Controller Object Reference") (DamageCauser :type "Actor Object Reference"))
  (set `self.Health` (- (`self.Health`) Damage))
  (`KismetSystemLibrary.PrintString` (`KismetStringLibrary.Conv_DoubleToString` (`self.Health`))))

(event `self.ReceiveTick`
  (params (DeltaSeconds :type "Float (single-precision)"))
  (bind _player (`self.Player`))
  (`|ExecutionSequence`
    (:`then_0`
      (if (<= (`self.Health`) 0.0)
        (`/Engine/EditorBlueprintResources/StandardMacros.DoOnce` false
          (:`Completed`
            (set `self.IsTrack` false)
            (set `/Game/MyTPS/Assets/Enemy/zombie/AB_Zombie.IsDead` true (`self.Enemy`))
            (set `/Game/MyTPS/Assets/Blueprints/BP_BaseCharacter.Score` (+ (`/Game/MyTPS/Assets/Blueprints/BP_BaseCharacter.Score` _player) 1) _player)
            (`KismetSystemLibrary.Delay` 3.0)
            (`self.K2_DestroyActor`)))))
    (:`then_1`
      (if (`self.IsTrack`)
        (`AIBlueprintHelperLibrary.SimpleMoveToActor` (`AIBlueprintHelperLibrary.GetAIController` self) (`self.Player`))
        (else
          (`MovementComponent.StopMovementImmediately` (`self.CharacterMovement`)))))
    (:`then_2`
      (if (and (`/Game/MyTPS/Assets/Enemy/zombie/AB_Zombie.IsHit` (`self.Enemy`)) (`self.IsAttack`))
        (`GameplayStatics.ApplyDamage` (`self.Player`) 30.0)
        (set `/Game/MyTPS/Assets/Enemy/zombie/AB_Zombie.IsHit` false (`self.Enemy`))))))

(event `self.Box.OnComponentBeginOverlap`
  (params (OverlappedComponent :type "PrimitiveComponent Object Reference") (OtherActor :type "Actor Object Reference") (OtherComp :type "PrimitiveComponent Object Reference") (OtherBodyIndex :type Integer) (bFromSweep :type Boolean) (SweepResult :type "HitResult Structure (by ref)"))
  (set `self.IsAttack` true)
  (if (`self.IsAttack`) :!label _label
    (set `self.IsTrack` false)
    (set `/Game/MyTPS/Assets/Enemy/zombie/AB_Zombie.IsAttacking` true (`self.Enemy`))
    (`KismetSystemLibrary.Delay` 1.0)
    (goto _label)))

(event `self.Box.OnComponentEndOverlap`
  (params (OverlappedComponent :type "PrimitiveComponent Object Reference") (OtherActor :type "Actor Object Reference") (OtherComp :type "PrimitiveComponent Object Reference") (OtherBodyIndex :type Integer))
  (set `self.IsAttack` false)
  (set `/Game/MyTPS/Assets/Enemy/zombie/AB_Zombie.IsAttacking` false (`self.Enemy`))
  (set `self.IsTrack` true))

(event `self.Sphere.OnComponentBeginOverlap`
  (params (OverlappedComponent :type "PrimitiveComponent Object Reference") (OtherActor :type "Actor Object Reference") (OtherComp :type "PrimitiveComponent Object Reference") (OtherBodyIndex :type Integer) (bFromSweep :type Boolean) (SweepResult :type "HitResult Structure (by ref)"))
  (set `self.IsTrack` true)
  (set `/Game/MyTPS/Assets/Enemy/zombie/AB_Zombie.IsTrack` true (`self.Enemy`)))

(event `self.Sphere.OnComponentEndOverlap`
  (params (OverlappedComponent :type "PrimitiveComponent Object Reference") (OtherActor :type "Actor Object Reference") (OtherComp :type "PrimitiveComponent Object Reference") (OtherBodyIndex :type Integer))
  (set `self.IsTrack` false)
  (set `/Game/MyTPS/Assets/Enemy/zombie/AB_Zombie.IsTrack` false (`self.Enemy`)))

(fn `UserConstructionScript`)