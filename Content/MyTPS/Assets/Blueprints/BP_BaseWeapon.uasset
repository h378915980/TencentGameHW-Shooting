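; Base weapon actor for a shooter, handling pickup, automatic fire and projectile spawning.
; Firing plays character and weapon montages; the weapon montage's blend-out spawns a projectile, shakes the camera and repeats while the trigger is held and rounds remain.
; Projectiles launch from the muzzle toward the character's look-at point, or straight along the muzzle at extreme yaw.
; Pickup stores the owner, disables physics and collision, and derives an aim offset from the sight socket.
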(event `self.ReceiveBeginPlay`)

(event `/Game/MyTPS/Assets/Blueprints/BPI_Weapons.FirePressed`
  (if (> (`self.RoundsinChamber`) 0)
    (`self.Fire`)))

(event `RepeatFire`
  (bind (_returnvalue_location _returnvalue_rotation _returnvalue_scale) (`KismetMathLibrary.BreakTransform` (`SceneComponent.GetSocketTransform` (`self.SkeletalMesh`) "Muzzle" "RTS_World")))
  (`|PlayMontage` (`Character.Mesh` (`self.Owning Character`)) "/Game/MyTPS/Assets/Character/Animation/A_2HW_ADS_Fire_Montage.A_2HW_ADS_Fire_Montage" :!label _label
    (:`then`
      (`|PlayMontage` (`self.SkeletalMesh`) "/Game/MyTPS/Assets/Weapons/AR/A_AR_Fire_Montage.A_AR_Fire_Montage" 2.0
        (:`OnBlendOut`
          (`self.Should Repeat Check`)
          (`PlayerCameraManager.StartCameraShake` :`self` (`GameplayStatics.GetPlayerCameraManager` 0) :`ShakeClass` "/Game/MyTPS/Assets/Blueprints/BP_CameraShake.BP_CameraShake_C")
          (bind _returnvalue (`|SpawnActorFromClass` "/Game/MyTPS/Assets/Blueprints/BP_BaseProjectile.BP_BaseProjectile_C" (`KismetMathLibrary.MakeTransform` _returnvalue_location _returnvalue_rotation (* _returnvalue_scale 3.0)) "AlwaysSpawn" "OverrideRootScale" self null))
          (set `MovementComponent.Velocity` (* (`KismetMathLibrary.SelectVector` (`KismetMathLibrary.GetForwardVector` (`SceneComponent.GetSocketRotation` (`self.SkeletalMesh`) "Muzzle")) (`KismetMathLibrary.Normal` (- (`/Game/MyTPS/Assets/Blueprints/BP_BaseCharacter.LookAtPoint` (`self.Owning Character`)) (`SceneComponent.GetSocketLocation` (`self.SkeletalMesh`) "Muzzle"))) (>= (`KismetMathLibrary.Abs` (`/Game/MyTPS/Assets/Blueprints/BP_BaseCharacter.Yaw` (`self.Owning Character`))) 90.0)) (`self.MuzzleVelocity`)) (`/Game/MyTPS/Assets/Blueprints/BP_BaseProjectile.ProjectileMovement` _returnvalue)))))))

(event `Fire`
  (set `self.Firing` true)
  (goto _label))

(event `FireRelease`
  (set `self.Firing` false))

(event `/Game/MyTPS/Assets/Blueprints/BPI_Weapons.GetWeapon`
  (params (OwningCharacter :type "/Game/MyTPS/Assets/Blueprints/BP_BaseCharacter Object Reference"))
  (set `self.Owning Character` OwningCharacter)
  (`PrimitiveComponent.SetSimulatePhysics` (`self.SkeletalMesh`) false)
  (`PrimitiveComponent.SetCollisionEnabled` (`self.SkeletalMesh`) "NoCollision")
  (set `self.AimBaselineOffset` (- (`KismetAnimationLibrary.K2_DistanceBetweenTwoSocketsAndMapRange` (`self.SkeletalMesh`) "Root" "RTS_World" "Sight" "RTS_World") 13.5)))

(fn `GetWeaponPanelInfo`
  (returns (Weapon :type "/Game/MyTPS/Assets/Blueprints/BP_BaseWeapon Object Reference") (WeaponType :type "/Game/MyTPS/Assets/Blueprints/EWeaponType Enum"))
  (return self (`self.WeaponType`)))

(fn `Should Repeat Check`
  (if (and (`self.Firing`) (> (`self.RoundsinChamber`) 0))
    (`self.RepeatFire`)))

(fn `UserConstructionScript`)