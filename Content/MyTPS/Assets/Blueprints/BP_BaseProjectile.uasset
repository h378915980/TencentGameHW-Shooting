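; BP_BaseProjectile is a base projectile that damages what it hits and leaves a bullet hole.
; When its StaticMesh overlaps an actor other than its owner, it applies point damage using the reversed velocity as the hit direction.
; It then spawns a short-lived bullet hole decal at the sweep's impact point, oriented to the surface normal, and destroys itself.
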(event `self.StaticMesh.OnComponentBeginOverlap`
  (params (OverlappedComponent :type "PrimitiveComponent Object Reference") (OtherActor :type "Actor Object Reference") (OtherComp :type "PrimitiveComponent Object Reference") (OtherBodyIndex :type Integer) (bFromSweep :type Boolean) (SweepResult :type "HitResult Structure (by ref)"))
  (bind (_hitresult_bblockinghit _hitresult_binitialoverlap _hitresult_time _hitresult_distance _hitresult_location _hitresult_impactpoint _hitresult_normal _hitresult_impactnormal) (`GameplayStatics.BreakHitResult` (`self.HitResult`)))
  (set `self.HitResult` SweepResult)
  (if (!= OtherActor (`self.GetOwner`))
    (`GameplayStatics.ApplyPointDamage` OtherActor 10.0 (* (`KismetMathLibrary.Normal` (`self.GetVelocity`)) -1.0) SweepResult)
    (`GameplayStatics.SpawnDecalAtLocation` "/Game/MyTPS/Assets/Weapons/M_BulletHole_Inst1.M_BulletHole_Inst1" (10.0 10.0 10.0) _hitresult_impactpoint (`KismetMathLibrary.Conv_VectorToRotator` _hitresult_impactnormal) 5.0)
    (`self.K2_DestroyActor`)))

(fn `UserConstructionScript`)